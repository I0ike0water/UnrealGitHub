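; Whack-a-mole style table actor that pops a random bird or pig up from one of ten torus holes.
; BeginPlay or MoleGameStart waits briefly, then SpawnActorFromTorus picks a random torus and one of three classes, spawning it just below that torus.
; The spawned BP_MoleGameActor gets a reference to this table, and a timeline moves it along Z, scaled by delta time.
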(event Custom|MoleGameStart
  (bind _currentspawnactor (Variables|Default|GetCurrentSpawnActor))
  (bind _returnvalue (Transformation|GetActorLocation _currentspawnactor))
  (Utilities|FlowControl|Delay 1.0)
  (CallFunction|SpawnActorfromTorus)
  (bind _asbp_mole_game_actor (Utilities|Casting|CastToBP_MoleGameActor _currentspawnactor))
  (Variables|/Game/__Actor/__MoleGame/BP_MoleGameActor.BP_MoleGameActor_C|SetBP_Table _asbp_mole_game_actor self)
  (bind _새_트랙_1 (Timeline|Current%20Spawn%20Actor%20Z%20move PlayFromStart)
    (:Update
      (Transformation|SetActorLocation _currentspawnactor (Math|Vector|MakeVector (.x _returnvalue) (.y _returnvalue) (+ (.z _returnvalue) (* _새_트랙_1 (Utilities|Time|GetWorldDeltaSeconds)))) false false))))

(event EventBeginPlay
  (bind _currentspawnactor (Variables|Default|GetCurrentSpawnActor))
  (bind _returnvalue (Transformation|GetActorLocation _currentspawnactor))
  (Utilities|FlowControl|Delay 1.0)
  (CallFunction|SpawnActorfromTorus)
  (bind _asbp_mole_game_actor (Utilities|Casting|CastToBP_MoleGameActor _currentspawnactor))
  (Variables|/Game/__Actor/__MoleGame/BP_MoleGameActor.BP_MoleGameActor_C|SetBP_Table _asbp_mole_game_actor self)
  (bind _새_트랙_1 (Timeline|Current%20Spawn%20Actor%20Z%20move PlayFromStart)
    (:Update
      (Transformation|SetActorLocation _currentspawnactor (Math|Vector|MakeVector (.x _returnvalue) (.y _returnvalue) (+ (.z _returnvalue) (* _새_트랙_1 (Utilities|Time|GetWorldDeltaSeconds)))) false false))))

(fn ConstructionScript)

(fn SpawnActorfromTorus
  (switch int (Math|Random|RandomInteger 10)
    (:0
      (Variables|Default|SetCurrentTorus (Variables|Default|GetTorus1)))
    (:1
      (Variables|Default|SetCurrentTorus (Variables|Default|GetTorus2)))
    (:2
      (Variables|Default|SetCurrentTorus (Variables|Default|GetTorus3)))
    (:3
      (Variables|Default|SetCurrentTorus (Variables|Default|GetTorus4)))
    (:4
      (Variables|Default|SetCurrentTorus (Variables|Default|GetTorus5)))
    (:5
      (Variables|Default|SetCurrentTorus (Variables|Default|GetTorus6)))
    (:6
      (Variables|Default|SetCurrentTorus (Variables|Default|GetTorus7)))
    (:7
      (Variables|Default|SetCurrentTorus (Variables|Default|GetTorus8)))
    (:8
      (Variables|Default|SetCurrentTorus (Variables|Default|GetTorus9)))
    (:9
      (Variables|Default|SetCurrentTorus (Variables|Default|GetTorus10))))
  (Variables|Default|SetCurrentTorusLocation (Transformation|GetWorldLocation (Variables|Default|GetCurrentTorus)))
  (switch int (Math|Random|RandomInteger 3)
    (:0
      (Variables|Default|SetCurrentSpawnActorClass "/Game/__Actor/__MoleGame/BP_Bird1.BP_Bird1_C"))
    (:1
      (Variables|Default|SetCurrentSpawnActorClass "/Game/__Actor/__MoleGame/BP_Bird2.BP_Bird2_C"))
    (:2
      (Variables|Default|SetCurrentSpawnActorClass "/Game/__Actor/__MoleGame/BP_Pig.BP_Pig_C")))
  (bind _returnvalue (Game|SpawnActorfromClass (Variables|Default|GetCurrentSpawnActorClass) (Math|Transform|MakeTransform (+ (Variables|Default|GetCurrentTorusLocation) "0.000000,0.000000,-20.000000") "0.000000,90.000000,-20.000000" "1.200000,1.200000,1.200000") "Undefined" "MultiplyWithRoot" 0 0))
  (Variables|Default|SetCurrentSpawnActor _returnvalue))