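; BP_DoorToMain is a door actor that rises once the mole game ends, presumably opening the way to the main hall.
; Shortly after BeginPlay, it reaches the mole game table's timer widget through BP_GameInstance and binds EndGame to its game-over event.
; After a brief delay, EndGame plays a timeline that adds its track value, scaled by delta seconds, to the actor's Z location each update.
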(event Custom|End%20Game
  (bind _returnvalue (Transformation|GetActorLocation))
  (Utilities|FlowControl|Delay 2.0)
  (bind _새_트랙_0 (Timeline|타임라인 Play)
    (:Update
      (Transformation|SetActorLocation (Math|Vector|MakeVector (.x _returnvalue) (.y _returnvalue) (+ (.z _returnvalue) (* _새_트랙_0 (Utilities|Time|GetWorldDeltaSeconds)))) false false))))

(event EventBeginPlay
  (|CallParentFunction)
  (Utilities|FlowControl|Delay 2.0)
  (bind _asbp_game_instance (Utilities|Casting|CastToBP_GameInstance (Game|GetGameInstance)))
  (bind _aswbp_mole_game_timer (Utilities|Casting|CastToWBP_MoleGameTimer (UserInterface|GetWidget (Variables|/Game/__Actor/__MoleGame/BP_MoleTable.BP_MoleTable_C|GetTimer (Variables|/Game/__GameInstance/BP_GameInstance.BP_GameInstance_C|GetMoleGameTable _asbp_game_instance)))))
  (EventDispatchers|BindEventtoMoleGameOver _aswbp_mole_game_timer (delegate Custom|End%20Game)))

(event Collision|EventActorBeginOverlap
  (params (OtherActor :type Actor%20Object%20Reference))
  (|CallParentFunction OtherActor) ; 지금 이 노드는 비활성 상태입니다. \n핀을 끌어서 다른 노드를 연결하면 활성화됩니다.
)

(event EventTick
  (params (DeltaSeconds :type Float%20%28single-precision%29))
  (|CallParentFunction DeltaSeconds) ; 지금 이 노드는 비활성 상태입니다. \n핀을 끌어서 다른 노드를 연결하면 활성화됩니다.
)

(fn ConstructionScript
  (|CallParentFunction))