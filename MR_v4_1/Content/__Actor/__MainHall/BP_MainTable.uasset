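; Main hall table whose button launches the VR Mole game.
; BeginPlay spawns the mole table below it; the first button overlap turns the button yellow and starts a timeline-animated press.
; Chained timelines and delays then move and hide the main table, swap the hall pawn for the mole-game pawn, and move the mole table.
; Finally, it spawns and moves a tutorial actor, adds a hit collision and makes it hittable.
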(event OnComponentBeginOverlap(MoleCollision)
  (params (OverlappedComponent :type Primitive%20Component%20Object%20Reference) (OtherActor :type Actor%20Object%20Reference) (OtherComp :type Primitive%20Component%20Object%20Reference) (OtherBodyIndex :type Integer) (bFromSweep :type Boolean) (SweepResult :type Hit%20Result%20Structure%20%28by%20ref%29))
  (bind _molebutton (Variables|Default|GetMoleButton))
  (bind _relativelocation (Variables|/Script/Engine.SceneComponent|GetRelativeLocation _molebutton))
  (Utilities|FlowControl|DoOnce false
    (:Completed
      (if (not (Variables|Default|GetIsGameStart))
        (Variables|Default|SetIsGameStart true)
        (Utilities|Casting|CastToBP_VR_Hall_v1 OtherActor)
        (Rendering|Material|SetMaterial (Variables|Default|GetMoleButton) 0 "/Game/__Material/MAT_Yellow.MAT_Yellow")
        (bind _새_트랙_0 (Timeline|타임라인_1 PlayFromStart)
          (:Update
            (Transformation|SetRelativeLocation _molebutton (Math|Vector|MakeVector (.x _relativelocation) (.y _relativelocation) (+ _새_트랙_0 (Variables|Default|GetStartLocation))) false false))
          (:Finished
            (Utilities|FlowControl|Delay 1.0)
            (CallFunction|GameReady)
            (CallFunction|ChangeMolePawn)
            (Utilities|FlowControl|Delay 1.0)
            (CallFunction|PlayMole)))))))

(event OnComponentEndOverlap(MoleCollision)
  (params (OverlappedComponent :type Primitive%20Component%20Object%20Reference) (OtherActor :type Actor%20Object%20Reference) (OtherComp :type Primitive%20Component%20Object%20Reference) (OtherBodyIndex :type Integer)))

(event Custom|Game%20End
  (Timeline|타임라인_0 Play))

(event Custom|Game%20Ready
  (bind _defaultsceneroot (Variables|Default|GetDefaultSceneRoot))
  (bind _returnvalue (Transformation|GetWorldLocation _defaultsceneroot))
  (bind _새_트랙_0 (Timeline|멜트다운 Play)
    (:Update
      (Transformation|SetWorldLocation _defaultsceneroot (Math|Vector|MakeVector (.x _returnvalue) (.y _returnvalue) (+ _새_트랙_0 (Variables|Default|GetStartTableLocationZ))) false false))
    (:Finished
      (Development|SetHiddeninGame _defaultsceneroot true false))))

(event Custom|PlayMole
  (bind _moletable (Variables|Default|GetMoleTable))
  (bind _defaultsceneroot (Variables|/Game/__Actor/__MoleGame/BP_MoleTable.BP_MoleTable_C|GetDefaultSceneRoot _moletable))
  (bind _returnvalue (Transformation|GetWorldLocation _defaultsceneroot))
  (bind _새_트랙_0 (Timeline|타임라인_2 Play)
    (:Update
      (Transformation|SetWorldLocation _defaultsceneroot (Math|Vector|MakeVector (.x _returnvalue) (.y _returnvalue) _새_트랙_0) false false))
    (:Finished
      (bind _returnvalue_2 (Game|SpawnActorfromClass "/Game/__UI/GameUI/Tuto1_0/BP_Tuto1_0.BP_Tuto1_0_C" (Math|Transform|MakeTransform (+ (Transformation|GetWorldLocation _defaultsceneroot) "45.000000,60.000000,0.000000") "0.000000,-90.000000,0.000000" "0.900000,0.900000,0.900000") "AlwaysSpawn" "MultiplyWithRoot" 0 0))
      (Variables|/Game/__Actor/__MoleGame/BP_MoleGameActor.BP_MoleGameActor_C|SetIs%20Hitable _returnvalue_2 false)
      (bind _output_get (Variables|Default|SetBP_Tuto1 _returnvalue_2))
      (bind _새_트랙_0_2 (Timeline|타임라인_3 Play)
        (:Update
          (Transformation|SetWorldLocation (Variables|/Script/Engine.Actor|GetRootComponent _output_get) (Math|Vector|MakeVector (.x (Transformation|GetWorldLocation (Variables|/Script/Engine.Actor|GetRootComponent _output_get))) (.y (Transformation|GetWorldLocation (Variables|/Script/Engine.Actor|GetRootComponent _output_get))) _새_트랙_0_2) false false))
        (:Finished
          (Game|SpawnActorfromClass "/Game/__Actor/__MoleGame/BP_HitableCollision.BP_HitableCollision_C" (Math|Transform|MakeTransform (Math|Vector|MakeVector (.x (Transformation|GetWorldLocation (Variables|/Script/Engine.Actor|GetRootComponent _output_get))) (.y (Transformation|GetWorldLocation (Variables|/Script/Engine.Actor|GetRootComponent _output_get))) (+ (.z (Transformation|GetWorldLocation (Variables|/Script/Engine.Actor|GetRootComponent _output_get))) -55.0)) "0, 0, 0" "1.000000,1.000000,1.000000") "Undefined" "MultiplyWithRoot" 0 0)
          (Variables|/Game/__Actor/__MoleGame/BP_MoleGameActor.BP_MoleGameActor_C|SetIs%20Hitable (Variables|Default|GetBP_Tuto1) true))))))

(event Custom|ChangeMolePawn
  (bind _returnvalue (Game|Player|GetPlayerPawn 0))
  (bind _returnvalue_2 (Game|SpawnActorfromClass "/Game/__Actor/BP_VR_MoleGame_v1.BP_VR_MoleGame_v1_C" (Math|Transform|MakeTransform (Transformation|GetActorLocation _returnvalue) (Transformation|GetActorRotation _returnvalue) "1.000000,1.000000,1.000000") "AlwaysSpawn" "MultiplyWithRoot" 0 0))
  (Actor|DestroyActor (Game|Player|GetPlayerPawn 0))
  (Pawn|Possess (Game|GetPlayerController 0) _returnvalue_2))

(event EventBeginPlay
  (bind _defaultsceneroot (Variables|Default|GetDefaultSceneRoot))
  (Variables|Default|SetStartTableLocationZ (.z (Transformation|GetWorldLocation _defaultsceneroot)))
  (bind _returnvalue (Game|SpawnActorfromClass "/Game/__Actor/__MoleGame/BP_MoleTable.BP_MoleTable_C" (Math|Transform|MakeTransform (+ (Transformation|GetWorldLocation _defaultsceneroot) "-40.000000,-40.000000,-200.000000") "0.000000,-90.000000,0.000000" "0.800000,0.800000,0.800000") "Undefined" "MultiplyWithRoot" 0 0))
  (Variables|Default|SetMoleTable _returnvalue))

(event Collision|EventActorBeginOverlap
  (params (OtherActor :type Actor%20Object%20Reference)))

(event EventTick
  (params (DeltaSeconds :type Float%20%28single-precision%29)))

(fn ConstructionScript)