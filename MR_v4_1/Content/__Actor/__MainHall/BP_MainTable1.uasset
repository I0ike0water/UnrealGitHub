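; VR main hall table that selects and launches the Mole and Slice minigames.
; The WBP_Swipe screen snaps between three pages, and a post-tutorial button press reads its position, the third page temporarily falling back to Mole.
; Timelines sink the table and raise the game's actors, while the player pawn is replaced per game.
; BackToMain restores table and hall pawn, revealing gender-based avatars once both score thresholds are passed.
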(event OnComponentBeginOverlap(ButtonCollision)
  (params (OverlappedComponent :type Primitive%20Component%20Object%20Reference) (OtherActor :type Actor%20Object%20Reference) (OtherComp :type Primitive%20Component%20Object%20Reference) (OtherBodyIndex :type Integer) (bFromSweep :type Boolean) (SweepResult :type Hit%20Result%20Structure%20%28by%20ref%29))
  (bind _button (Variables|Default|GetButton))
  (bind _relativelocation (Variables|/Script/Engine.SceneComponent|GetRelativeLocation _button))
  (Utilities|Casting|CastToBP_VR_Hall_v1 OtherActor)
  (if (Variables|/Game/__GameInstance/BP_GameInstance.BP_GameInstance_C|GetMainTutoEnd (Variables|Default|GetGame%20Instance))
    (Utilities|FlowControl|DoOnce false
      (:Completed
        (if (not (Variables|Default|GetIsGameStart))
          (Variables|Default|SetIsGameStart true)
          (Rendering|Material|SetMaterial (Variables|Default|GetButton) 0 "/Game/__Material/MAT_Yellow.MAT_Yellow")
          (bind _새_트랙_0 (Timeline|타임라인_1 PlayFromStart)
            (:Update
              (Transformation|SetRelativeLocation _button (Math|Vector|MakeVector (.x _relativelocation) (.y _relativelocation) (+ _새_트랙_0 (Variables|Default|GetStartLocation))) false false))
            (:Finished
              (Utilities|FlowControl|Delay 1.0)
              (CallFunction|GameReady)
              (bind _aswbp_swipe (Utilities|Casting|CastToWBP_Swipe (UserInterface|GetWidget (Variables|Default|GetGameScreen))))
              (if (> (.x (.translation (Variables|/Script/UMG.Widget|GetRenderTransform (Variables|/Game/__UI/GameUI/MainUI/WBP_Swipe.WBP_Swipe_C|GetHorizontalBox_27 _aswbp_swipe)))) -7.5e+02)
                (CallFunction|ChangeMolePawn)
                (Utilities|FlowControl|Delay 1.0)
                (CallFunction|PlayMole)
                (elif (> (.x (.translation (Variables|/Script/UMG.Widget|GetRenderTransform (Variables|/Game/__UI/GameUI/MainUI/WBP_Swipe.WBP_Swipe_C|GetHorizontalBox_27 _aswbp_swipe)))) -2.25e+03)
                  (CallFunction|ChangeSlicePawn)
                  (Utilities|FlowControl|Delay 1.0)
                  (CallFunction|PlaySlice)
                  (else
                    ;[1 1 1] 임시
                    (CallFunction|ChangeMolePawn)
                    (Utilities|FlowControl|Delay 1.0)
                    (CallFunction|PlayMole)))))))))))

(event OnComponentEndOverlap(ButtonCollision)
  (params (OverlappedComponent :type Primitive%20Component%20Object%20Reference) (OtherActor :type Actor%20Object%20Reference) (OtherComp :type Primitive%20Component%20Object%20Reference) (OtherBodyIndex :type Integer)))

(event Custom|Past%20Game)

(event Custom|Game%20Ready
  (bind _button (Variables|Default|GetButton))
  (bind _defaultsceneroot (Variables|Default|GetDefaultSceneRoot))
  (bind _returnvalue (Transformation|GetWorldLocation _defaultsceneroot))
  (bind _relativelocation (Variables|/Script/Engine.SceneComponent|GetRelativeLocation _button))
  (bind _새_트랙_0 (Timeline|멜트다운 PlayFromStart)
    (:Update
      (Transformation|SetWorldLocation _defaultsceneroot (Math|Vector|MakeVector (.x _returnvalue) (.y _returnvalue) (+ _새_트랙_0 (Variables|Default|GetStartTableLocationZ))) false false))
    (:Finished
      (Development|SetHiddeninGame _defaultsceneroot true true)
      (Rendering|Material|SetMaterial (Variables|Default|GetButton) 0 "/Game/__Material/MAT_Red.MAT_Red")
      (bind _새_트랙_0_2 (Timeline|타임라인_7 ReverseFromEnd)
        (:Update
          (Transformation|SetRelativeLocation _button (Math|Vector|MakeVector (.x _relativelocation) (.y _relativelocation) (+ _새_트랙_0_2 (Variables|Default|GetStartLocation))) false false)
          (Variables|Default|SetIsGameStart false))))))

(event Custom|Show%20Avatar
  (bind _game_instance (Variables|Default|GetGame%20Instance))
  (bind _game_instance_2 (Variables|Default|GetGame%20Instance))
  (bind _game_instance_3 (Variables|Default|GetGame%20Instance))
  (bind _pawnactor (Variables|/Game/__GameInstance/BP_GameInstance.BP_GameInstance_C|GetPawnActor _game_instance))
  (bind _pawnactor_2 (Variables|/Game/__GameInstance/BP_GameInstance.BP_GameInstance_C|GetPawnActor _game_instance_3))
  (bind _output (Utilities|Array|Get(acopy) _pawnactor 3))
  (bind _output_2 (Utilities|Array|Get(acopy) _pawnactor 2))
  (bind _output_3 (Utilities|Array|Get(acopy) _pawnactor_2))
  (bind _output_4 (Utilities|Array|Get(acopy) _pawnactor_2 1))
  (if (and (> (Variables|/Game/__GameInstance/BP_GameInstance.BP_GameInstance_C|GetFirstGameScore _game_instance_2) 49.0) (> (Variables|/Game/__GameInstance/BP_GameInstance.BP_GameInstance_C|GetSecondGameScore _game_instance_2) 99.0))
    (if (Utilities|Enum|Equal(Enum) (Variables|/Game/__GameInstance/BP_GameInstance.BP_GameInstance_C|GetGender _game_instance_2) "male")
      (bind _asbp_male (Utilities|Casting|CastToBP_Male _output_3))
      (Default|GetHeight _asbp_male)
      (Rendering|SetActorHiddenInGame _output_3 false)
      (bind _asbp_male_random (Utilities|Casting|CastToBP_MaleRandom _output_4))
      (Default|GetHeight _asbp_male_random)
      (Rendering|SetActorHiddenInGame _output_4 false)
      (else
        (bind _asbp_female_random (Utilities|Casting|CastToBP_FemaleRandom _output)
          (:then
            (Default|GetHeight _asbp_female_random)
            (Rendering|SetActorHiddenInGame _output false))
          (:CastFailed
            (bind _asbp_female (Utilities|Casting|CastToBP_Female _output_2))
            (Default|GetHeight _asbp_female)
            (Rendering|SetActorHiddenInGame _output_2 false)))))))

(event Custom|Press%20X%20to%20Joy
  (bind _button (Variables|Default|GetButton))
  (bind _relativelocation (Variables|/Script/Engine.SceneComponent|GetRelativeLocation _button))
  (if (Variables|/Game/__GameInstance/BP_GameInstance.BP_GameInstance_C|GetMainTutoEnd (Variables|Default|GetGame%20Instance))
    (Utilities|FlowControl|DoOnce false
      (:Completed
        (if (not (Variables|Default|GetIsGameStart))
          (Variables|Default|SetIsGameStart true)
          (Rendering|Material|SetMaterial (Variables|Default|GetButton) 0 "/Game/__Material/MAT_Yellow.MAT_Yellow")
          (bind _새_트랙_0 (Timeline|타임라인_1 PlayFromStart)
            (:Update
              (Transformation|SetRelativeLocation _button (Math|Vector|MakeVector (.x _relativelocation) (.y _relativelocation) (+ _새_트랙_0 (Variables|Default|GetStartLocation))) false false))
            (:Finished
              (Utilities|FlowControl|Delay 1.0)
              (CallFunction|GameReady)
              (bind _aswbp_swipe (Utilities|Casting|CastToWBP_Swipe (UserInterface|GetWidget (Variables|Default|GetGameScreen))))
              (if (> (.x (.translation (Variables|/Script/UMG.Widget|GetRenderTransform (Variables|/Game/__UI/GameUI/MainUI/WBP_Swipe.WBP_Swipe_C|GetHorizontalBox_27 _aswbp_swipe)))) -7.5e+02)
                (CallFunction|ChangeMolePawn)
                (Utilities|FlowControl|Delay 1.0)
                (CallFunction|PlayMole)
                (elif (> (.x (.translation (Variables|/Script/UMG.Widget|GetRenderTransform (Variables|/Game/__UI/GameUI/MainUI/WBP_Swipe.WBP_Swipe_C|GetHorizontalBox_27 _aswbp_swipe)))) -2.25e+03)
                  (CallFunction|ChangeSlicePawn)
                  (Utilities|FlowControl|Delay 1.0)
                  (CallFunction|PlaySlice)
                  (else
                    ;[1 1 1] 임시
                    (CallFunction|ChangeMolePawn)
                    (Utilities|FlowControl|Delay 1.0)
                    (CallFunction|PlayMole)))))))))))

(event Custom|PlayMole
  (bind _returnvalue (Game|SpawnActorfromClass "/Game/__Actor/__MoleGame/BP_MoleTable.BP_MoleTable_C" (Math|Transform|MakeTransform (+ (Transformation|GetWorldLocation (Variables|Default|GetDefaultSceneRoot)) (Math|Vector|MakeVector -4e+01 -4e+01 (+ (Variables|Default|GetStartTableLocationZ) -1.1e+02))) "0.000000,-90.000000,0.000000" "0.800000,0.800000,0.800000") "AlwaysSpawn" "MultiplyWithRoot" 0 0))
  (bind _output_get (Variables|Default|SetMoleTable _returnvalue))
  (Variables|/Game/__Actor/__MoleGame/BP_MoleTable.BP_MoleTable_C|SetMainTable _output_get self)
  (bind _새_트랙_0 (Timeline|타임라인_2 PlayFromStart)
    (:Update
      (Transformation|SetWorldLocation (Variables|/Game/__Actor/__MoleGame/BP_MoleTable.BP_MoleTable_C|GetDefaultSceneRoot (Variables|Default|GetMoleTable)) (Math|Vector|MakeVector (.x (Transformation|GetWorldLocation (Variables|/Game/__Actor/__MoleGame/BP_MoleTable.BP_MoleTable_C|GetDefaultSceneRoot (Variables|Default|GetMoleTable)))) (.y (Transformation|GetWorldLocation (Variables|/Game/__Actor/__MoleGame/BP_MoleTable.BP_MoleTable_C|GetDefaultSceneRoot (Variables|Default|GetMoleTable)))) _새_트랙_0) false false))
    (:Finished
      (bind _returnvalue_2 (Game|SpawnActorfromClass "/Game/__UI/GameUI/Tuto1_0/BP_Tuto1_0.BP_Tuto1_0_C" (Math|Transform|MakeTransform (+ (Transformation|GetWorldLocation (Variables|/Game/__Actor/__MoleGame/BP_MoleTable.BP_MoleTable_C|GetDefaultSceneRoot (Variables|Default|GetMoleTable))) "45.000000,30.000000,0.000000") "0.000000,-90.000000,0.000000" "0.800000,0.800000,0.800000") "AlwaysSpawn" "MultiplyWithRoot" 0 0))
      (Variables|/Game/__Actor/__MoleGame/BP_MoleGameActor.BP_MoleGameActor_C|SetIs%20Hitable _returnvalue_2 false)
      (bind _output_get_2 (Variables|Default|SetBP_Tuto1 _returnvalue_2))
      (bind _새_트랙_0_2 (Timeline|타임라인_3 PlayFromStart)
        (:Update
          (Transformation|SetWorldLocation (Variables|/Script/Engine.Actor|GetRootComponent _output_get_2) (Math|Vector|MakeVector (.x (Transformation|GetWorldLocation (Variables|/Script/Engine.Actor|GetRootComponent _output_get_2))) (.y (Transformation|GetWorldLocation (Variables|/Script/Engine.Actor|GetRootComponent _output_get_2))) _새_트랙_0_2) false false))
        (:Finished
          (bind _returnvalue_3 (Game|SpawnActorfromClass "/Game/__Actor/__MoleGame/BP_HitableCollision.BP_HitableCollision_C" (Math|Transform|MakeTransform (Math|Vector|MakeVector (.x (Transformation|GetWorldLocation (Variables|/Script/Engine.Actor|GetRootComponent _output_get_2))) (.y (Transformation|GetWorldLocation (Variables|/Script/Engine.Actor|GetRootComponent _output_get_2))) (+ (.z (Transformation|GetWorldLocation (Variables|/Script/Engine.Actor|GetRootComponent _output_get_2))) -45.0)) "0, 0, 0" "1.000000,1.000000,1.000000") "AlwaysSpawn" "MultiplyWithRoot" 0 0))
          (Variables|/Game/__Actor/__MoleGame/BP_MoleGameActor.BP_MoleGameActor_C|SetIs%20Hitable (Variables|Default|GetBP_Tuto1) true))))))

(event Custom|ChangeMolePawn
  (bind _returnvalue (Game|Player|GetPlayerPawn 0))
  ;[1 1 1] Pawn 변경
  (bind _returnvalue_2 (Game|SpawnActorfromClass "/Game/__Actor/BP_VR_MoleGame_v1.BP_VR_MoleGame_v1_C" (Math|Transform|MakeTransform (Transformation|GetActorLocation _returnvalue) (Transformation|GetActorRotation _returnvalue) "1.000000,1.000000,1.000000") "AlwaysSpawn" "MultiplyWithRoot" 0 0))
  (Actor|DestroyActor (Game|Player|GetPlayerPawn 0))
  (Pawn|Possess (Game|GetPlayerController 0) _returnvalue_2))

(event Custom|GameScreen%20Set
  (if (< -1e+03 (.x (.translation (Variables|/Script/UMG.Widget|GetRenderTransform (Variables|/Game/__UI/GameUI/MainUI/WBP_Swipe.WBP_Swipe_C|GetHorizontalBox_27 (stale EventBeginPlay _aswbp_swipe))))))
    (bind _새_트랙_0 (Timeline|타임라인_4 PlayFromStart)
      (:Update
        (Class|Widget|SetRenderTransform (Variables|/Game/__UI/GameUI/MainUI/WBP_Swipe.WBP_Swipe_C|GetHorizontalBox_27 (stale EventBeginPlay _aswbp_swipe)) (Utilities|Struct|MakeWidgetTransform (Math|Vector2D|MakeVector2D (Math|Float|Lerp (.x (.translation (Variables|/Script/UMG.Widget|GetRenderTransform (Variables|/Game/__UI/GameUI/MainUI/WBP_Swipe.WBP_Swipe_C|GetHorizontalBox_27 (stale EventBeginPlay _aswbp_swipe))))) 0.0 _새_트랙_0) 0.0) "(X=1.000000,Y=1.000000)" "(X=0.000000,Y=0.000000)" 0.0)))
      (:Finished
        (Variables|/Game/__UI/GameUI/MainUI/WBP_Swipe.WBP_Swipe_C|SetisAdjusting (stale EventBeginPlay _aswbp_swipe) false :!label _label)))
    (elif (< -3e+03 (.x (.translation (Variables|/Script/UMG.Widget|GetRenderTransform (Variables|/Game/__UI/GameUI/MainUI/WBP_Swipe.WBP_Swipe_C|GetHorizontalBox_27 (stale EventBeginPlay _aswbp_swipe))))))
      (bind _새_트랙_0_2 (Timeline|타임라인_5 PlayFromStart)
        (:Update
          (Class|Widget|SetRenderTransform (Variables|/Game/__UI/GameUI/MainUI/WBP_Swipe.WBP_Swipe_C|GetHorizontalBox_27 (stale EventBeginPlay _aswbp_swipe)) (Utilities|Struct|MakeWidgetTransform (Math|Vector2D|MakeVector2D (Math|Float|Lerp (.x (.translation (Variables|/Script/UMG.Widget|GetRenderTransform (Variables|/Game/__UI/GameUI/MainUI/WBP_Swipe.WBP_Swipe_C|GetHorizontalBox_27 (stale EventBeginPlay _aswbp_swipe))))) -2e+03 _새_트랙_0_2) 0.0) "(X=1.000000,Y=1.000000)" "(X=0.000000,Y=0.000000)" 0.0)))
        (:Finished
          (goto _label)))
      (else
        (bind _새_트랙_0_3 (Timeline|타임라인_6 PlayFromStart)
          (:Update
            (Class|Widget|SetRenderTransform (Variables|/Game/__UI/GameUI/MainUI/WBP_Swipe.WBP_Swipe_C|GetHorizontalBox_27 (stale EventBeginPlay _aswbp_swipe)) (Utilities|Struct|MakeWidgetTransform (Math|Vector2D|MakeVector2D (Math|Float|Lerp (.x (.translation (Variables|/Script/UMG.Widget|GetRenderTransform (Variables|/Game/__UI/GameUI/MainUI/WBP_Swipe.WBP_Swipe_C|GetHorizontalBox_27 (stale EventBeginPlay _aswbp_swipe))))) -4e+03 _새_트랙_0_3) 0.0) "(X=1.000000,Y=1.000000)" "(X=0.000000,Y=0.000000)" 0.0)))
          (:Finished
            (goto _label)))))))

(event Custom|ChangeSlicePawn
  (bind _returnvalue (Game|Player|GetPlayerPawn 0))
  ;[1 1 1] Pawn 변경
  (bind _returnvalue_2 (Game|SpawnActorfromClass "/Game/__Actor/BP_VR_Slice_v1.BP_VR_Slice_v1_C" (Math|Transform|MakeTransform (Transformation|GetActorLocation _returnvalue) (Transformation|GetActorRotation _returnvalue) "1.000000,1.000000,1.000000") "AlwaysSpawn" "MultiplyWithRoot" 0 0))
  (Actor|DestroyActor (Game|Player|GetPlayerPawn 0))
  (Pawn|Possess (Game|GetPlayerController 0) _returnvalue_2))

(event Custom|Play%20Slice
  (bind _returnvalue (Game|SpawnActorfromClass "/Game/__Actor/BP_Spawner.BP_Spawner_C" (Math|Transform|MakeTransform (+ (Transformation|GetWorldLocation (Variables|Default|GetDefaultSceneRoot)) "0.000000,-725.000000,-75.000000") "0, 0, 0" "1.000000,1.000000,1.000000") "AlwaysSpawn" "MultiplyWithRoot" 0 0))
  (bind _output_get (Variables|Default|SetSliceSpawner _returnvalue))
  (bind _output_get_2 (Variables|Default|SetSliceSpawnerLocationZ (.z (Transformation|GetWorldLocation (Variables|/Game/__Actor/BP_Spawner.BP_Spawner_C|GetDefaultSceneRoot _output_get)))))
  (Variables|/Game/__Actor/BP_Spawner.BP_Spawner_C|SetMainTable _returnvalue self)
  (bind _새_트랙_0 (Timeline|타임라인_8 PlayFromStart)
    (:Update
      (Transformation|SetWorldLocation (Variables|/Game/__Actor/BP_Spawner.BP_Spawner_C|GetDefaultSceneRoot _output_get) (Math|Vector|MakeVector (.x (Transformation|GetWorldLocation (Variables|/Game/__Actor/BP_Spawner.BP_Spawner_C|GetDefaultSceneRoot _output_get))) (.y (Transformation|GetWorldLocation (Variables|/Game/__Actor/BP_Spawner.BP_Spawner_C|GetDefaultSceneRoot _output_get))) (+ _새_트랙_0 _output_get_2)) false false))
    (:Finished
      (Game|SpawnActorfromClass "/Game/__UI/GameUI/Tuto2_0/BP_Tuto2_0.BP_Tuto2_0_C" (Math|Transform|MakeTransform "0, 0, 0" "0, 0, 0" "1.000000,1.000000,1.000000") "AlwaysSpawn" "MultiplyWithRoot" 0 0))))

(event Custom|ChangeHallPawn
  (bind _returnvalue (Game|Player|GetPlayerPawn 0))
  ;[1 1 1] Pawn 변경
  (bind _returnvalue_2 (Game|SpawnActorfromClass "/Game/__Actor/BP_VR_Hall_v1.BP_VR_Hall_v1_C" (Math|Transform|MakeTransform (Transformation|GetActorLocation _returnvalue) (Transformation|GetActorRotation _returnvalue) "1.000000,1.000000,1.000000") "AlwaysSpawn" "MultiplyWithRoot" 0 0))
  (Actor|DestroyActor (Game|Player|GetPlayerPawn 0))
  (Pawn|Possess (Game|GetPlayerController 0) _returnvalue_2))

(event Custom|Back%20To%20Main
  (bind _defaultsceneroot (Variables|Default|GetDefaultSceneRoot))
  (bind _button (Variables|Default|GetButton))
  (bind _returnvalue (Transformation|GetWorldLocation _defaultsceneroot))
  (bind _relativelocation (Variables|/Script/Engine.SceneComponent|GetRelativeLocation _button))
  (Development|SetHiddeninGame _defaultsceneroot false true)
  (Development|SetHiddeninGame (Variables|Default|GetButtonCollision) true false)
  (bind _새_트랙_0 (Timeline|타임라인_9 PlayFromStart)
    (:Update
      (Transformation|SetWorldLocation _defaultsceneroot (Math|Vector|MakeVector (.x _returnvalue) (.y _returnvalue) (+ _새_트랙_0 (Variables|Default|GetStartTableLocationZ))) false false))
    (:Finished
      (CallFunction|ChangeHallPawn)
      (Variables|Default|SetIsGameStart false)
      (CallFunction|ShowAvatar)
      (if (Utilities|IsValid (stale Custom|PlayMole _returnvalue_3))
        (Actor|DestroyActor (stale Custom|PlayMole _returnvalue_3))
        (Utilities|FlowControl|DoOnce false) ; enters at Reset
        (else
          (Utilities|FlowControl|DoOnce false) ; enters at Reset
        )))))

(event Custom|Next%20Game)

(event EventBeginPlay
  (Variables|Default|SetStartTableLocationZ (.z (Transformation|GetWorldLocation (Variables|Default|GetDefaultSceneRoot))))
  (bind _asbp_game_instance (Utilities|Casting|CastToBP_GameInstance (Game|GetGameInstance)))
  (bind _output_get (Variables|Default|SetGame%20Instance _asbp_game_instance))
  (Variables|/Game/__GameInstance/BP_GameInstance.BP_GameInstance_C|SetMainTable _output_get self)
  (bind _aswbp_swipe (Utilities|Casting|CastToWBP_Swipe (UserInterface|GetWidget (Variables|Default|GetGameScreen))))
  (EventDispatchers|BindEventtoConfirmGame _aswbp_swipe (delegate Custom|GameScreen%20Set)))

(fn ConstructionScript)