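; Server bridge actor that uploads a recorded WAV file to a remote server and stores the returned result as the player's gender.
; On BeginPlay it registers itself with BP_GameInstance as BPServer.
; SendFile sends a hard-coded local Test.wav to the GameInstance IP and port, then busy-waits on SendCheck.
; It then writes FinalResult to GameInstance.Gender and prints it on screen.
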(event Custom|Send%20File
  (bind _finalresult (Variables|Default|GetFinalResult))
  (Class|FileSend|SendFiletoServer (Variables|/Game/__GameInstance/BP_GameInstance.BP_GameInstance_C|GetIP (stale EventBeginPlay _output_get)) (Math|Conversions|ToInteger(Byte) (Variables|/Game/__GameInstance/BP_GameInstance.BP_GameInstance_C|GetPort (stale EventBeginPlay _output_get))) "C:\\Users\\ETRI\\Documents\\UnrealGitHub\\MR_v4_1\\Content\\__FileSave\\Test.wav")
  (while (== (Variables|Default|GetSendCheck) false)
    _)
  (Variables|/Game/__GameInstance/BP_GameInstance.BP_GameInstance_C|SetGender (stale EventBeginPlay _output_get) _finalresult)
  (Development|PrintString _finalresult true true "(R=0.000000,G=0.660000,B=1.000000,A=1.000000)" 12.0))

(event EventBeginPlay
  (bind _asbp_game_instance (Utilities|Casting|CastToBP_GameInstance (Game|GetGameInstance)))
  (bind _output_get (Variables|Default|SetGame%20Instance _asbp_game_instance))
  (Variables|/Game/__GameInstance/BP_GameInstance.BP_GameInstance_C|SetBP_Server _output_get self))

(fn ConstructionScript)