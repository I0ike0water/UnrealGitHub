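; Female avatar Blueprint that shows a rigged character with name-tag and physical-info widgets.
; On BeginPlay it registers itself in the third slot of the game instance's PawnActor array and hides itself.
; GetHeight reads the current height from ABP_Female and repositions the tag widget with a height-mapped offset that shrinks as height grows.
; It then labels the tag "Real" and refreshes the physical-info widget.
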(event Custom|Get%20Height
  (bind _widget (Variables|Default|GetWidget))
  (bind _asabp_female (Utilities|Casting|CastToABP_Female (Components|SkeletalMesh|GetAnimInstance (Variables|Default|Getrp_carla_rigged_001_ue4))))
  (Transformation|SetRelativeLocation _widget (Math|Vector|MakeVector 0.0 0.0 (+ (Variables|/Game/__Actor/__Avatar/ABP_Female.ABP_Female_C|GetCurrentHeight _asabp_female) (Math|Float|MapRangeClamped (Variables|/Game/__Actor/__Avatar/ABP_Female.ABP_Female_C|GetCurrentHeight _asabp_female) 1.2e+02 2.4e+02 75.0 2e+01))) false false)
  (bind _aswbp_avatar (Utilities|Casting|CastToWBP_Avatar (UserInterface|GetWidget _widget)))
  (Variables|/Script/UMG.TextBlock|SetText (Variables|/Game/__UI/HUD/WBP_Avatar.WBP_Avatar_C|GetTextBlock_52 _aswbp_avatar) "Real")
  (bind _aswbp_physical_info (Utilities|Casting|CastToWBP_PhysicalInfo (UserInterface|GetWidget (Variables|Default|GetInfoWidget))))
  (Default|UpdatePhysical _aswbp_physical_info))

(event EventBeginPlay
  (bind _self self)
  (bind _asbp_game_instance (Utilities|Casting|CastToBP_GameInstance (Game|GetGameInstance)))
  (Variables|/Game/__GameInstance/BP_GameInstance.BP_GameInstance_C|SetPawnActor _asbp_game_instance (Utilities|Array|MakeArray (Utilities|Array|Get(acopy) (Variables|/Game/__GameInstance/BP_GameInstance.BP_GameInstance_C|GetPawnActor _asbp_game_instance)) (Utilities|Array|Get(acopy) (Variables|/Game/__GameInstance/BP_GameInstance.BP_GameInstance_C|GetPawnActor _asbp_game_instance) 1) _self (Utilities|Array|Get(acopy) (Variables|/Game/__GameInstance/BP_GameInstance.BP_GameInstance_C|GetPawnActor _asbp_game_instance) 3)))
  (Rendering|SetActorHiddenInGame _self true))

(fn ConstructionScript)