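; Female random avatar actor that registers itself as the fourth entry in the game instance's PawnActor array and starts hidden.
; GetHeight reads height, sitting height and wingspan from ABP_FemaleRandom and passes them, with the female gender, to the WBP_PhysicalInfo widget.
; It also shifts the root vertically by an offset mapped from the current height.
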(event Custom|Get%20Height
  (bind _asabp_female_random (Utilities|Casting|CastToABP_FemaleRandom (Components|SkeletalMesh|GetAnimInstance (Variables|Default|Getrp_carla_rigged_001_ue4))))
  (bind _aswbp_physical_info (Utilities|Casting|CastToWBP_PhysicalInfo (UserInterface|GetWidget (Variables|Default|GetInfoWidget))))
  (Default|UpdateRandomPhysical _aswbp_physical_info (Variables|/Game/__Actor/__Avatar/ABP_FemaleRandom.ABP_FemaleRandom_C|GetCurrentHeight _asabp_female_random) (Variables|/Game/__Actor/__Avatar/ABP_FemaleRandom.ABP_FemaleRandom_C|GetCurrentSittingHeight _asabp_female_random) (Variables|/Game/__Actor/__Avatar/ABP_FemaleRandom.ABP_FemaleRandom_C|GetCurrentWingSpan _asabp_female_random))
  (Default|SetGender _aswbp_physical_info "female")
  (Transformation|AddWorldOffset (Variables|Default|GetDefaultSceneRoot) (Math|Vector|MakeVector 0.0 0.0 (Math|Float|MapRangeClamped (Variables|/Game/__Actor/__Avatar/ABP_FemaleRandom.ABP_FemaleRandom_C|GetCurrentHeight _asabp_female_random) 5e+01 2.5e+02 -2e+01 75.0)) false false))

(event EventBeginPlay
  (bind _self self)
  (bind _asbp_game_instance (Utilities|Casting|CastToBP_GameInstance (Game|GetGameInstance)))
  (Variables|/Game/__GameInstance/BP_GameInstance.BP_GameInstance_C|SetPawnActor _asbp_game_instance (Utilities|Array|MakeArray (Utilities|Array|Get(acopy) (Variables|/Game/__GameInstance/BP_GameInstance.BP_GameInstance_C|GetPawnActor _asbp_game_instance)) (Utilities|Array|Get(acopy) (Variables|/Game/__GameInstance/BP_GameInstance.BP_GameInstance_C|GetPawnActor _asbp_game_instance) 1) (Utilities|Array|Get(acopy) (Variables|/Game/__GameInstance/BP_GameInstance.BP_GameInstance_C|GetPawnActor _asbp_game_instance) 2) _self))
  (Rendering|SetActorHiddenInGame _self true))

(fn ConstructionScript)