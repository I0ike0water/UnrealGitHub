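; BP_Sliceable_Ori is a sliceable projectile actor, apparently for the VR slicing game.
; Construction copies its static mesh into a procedural mesh with collision, which moves along negative X each tick unless in tutorial or already sliced.
; Sliced plays one of two random sounds, enables gravity and schedules destruction.
; SpawnScore creates a score popup at the mesh, oriented using the VR pawn's camera.
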(event Custom|Spawn%20Score
  (params (ScoreNum :type Integer))
  (bind _asbp_vr_slice_v_1 (Utilities|Casting|CastToBP_VR_Slice_v1 (Game|Player|GetPlayerPawn 0)))
  (Game|SpawnActorfromClass "/Game/__UI/GameUI/Score/BP_PopUpScore.BP_PopUpScore_C" (Math|Transform|MakeTransform (Transformation|GetWorldLocation (Variables|Default|GetProceduralMesh)) (Math|Conversions|RotationFromXVector (* (Transformation|GetWorldRotation (Variables|/Game/__Actor/BP_VR_Slice_v1.BP_VR_Slice_v1_C|GetCamera _asbp_vr_slice_v_1)) -1.0)) "1.000000,1.000000,1.000000") "Undefined" "MultiplyWithRoot" 0 ScoreNum 0))

(event Custom|Destroy_Slice_obj
  (params (Duration :type Float%20%28single-precision%29))
  (Utilities|FlowControl|Delay Duration)
  (Actor|DestroyActor))

(event EventTick
  (params (DeltaSeconds :type Float%20%28single-precision%29))
  (if (not (Variables|Default|GetIsTuto))
    (if (not (Variables|Default|GetIsAlreadySliced))
      (Transformation|AddWorldOffset (Variables|Default|GetProceduralMesh) (Math|Vector|MakeVector (* -1.0 (Variables|Default|GetSpeed)) 0.0 0.0) false true))))

(fn ConstructionScript
  (Class|KismetProceduralMeshLibrary|CopyProceduralMeshfromStaticMeshComponent (Variables|Default|GetStaticMesh) 0 (Variables|Default|GetProceduralMesh) true)
  (Variables|Default|SetSlicedMaterial "/Game/VRTemplate/Materials/MI_Projectile.MI_Projectile"))

(fn Sliced
  (switch int (Math|Random|RandomInteger 2)
    (:0
      (Audio|PlaySoundatLocation "/Game/__Sound/__SoundCue/SliceSound1.SliceSound1" "0, 0, 0" "0, 0, 0" 1.0 1.0 0.0 0 0 0 0))
    (:1
      (Audio|PlaySoundatLocation "/Game/__Sound/__SoundCue/SliceSound2.SliceSound2" "0, 0, 0" "0, 0, 0" 1.0 1.0 0.0 0 0 0 0)))
  (Physics|SetEnableGravity (Variables|Default|GetProceduralMesh) true)
  (CallFunction|DestroySliceObj 3.0))