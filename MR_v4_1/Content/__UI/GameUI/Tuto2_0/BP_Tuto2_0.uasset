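; BP_Tuto2_0 is a tutorial UI actor, judging by its folder, whose procedural mesh floats in front of the VR player's view until it is sliced.
; Each Tick runs the parent logic, then places the mesh ahead of the BP_VR_Slice_v1 pawn's camera with matching rotation while IsAlreadySliced is false.
; Unconnected nodes hold an unused variant that spawns and positions a BP_Frame the same way.
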(event EventBeginPlay
  (|CallParentFunction))

(event EventTick
  (params (DeltaSeconds :type Float%20%28single-precision%29))
  (bind _proceduralmesh (Variables|Default|GetProceduralMesh))
  (|CallParentFunction DeltaSeconds)
  (if (not (Variables|Default|GetIsAlreadySliced))
    (bind _asbp_vr_slice_v_1 (Utilities|Casting|CastToBP_VR_Slice_v1 (Game|Player|GetPlayerPawn 0)))
    (Transformation|SetWorldLocation _proceduralmesh (+ (Transformation|GetWorldLocation (Variables|/Game/__Actor/BP_VR_Slice_v1.BP_VR_Slice_v1_C|GetCamera _asbp_vr_slice_v_1)) (* (Math|Vector|GetForwardVector (Variables|/Game/__Actor/BP_VR_Slice_v1.BP_VR_Slice_v1_C|GetCamera _asbp_vr_slice_v_1)) "120.000000,120.000000,50.000000")) false true)
    (Transformation|SetWorldRotation _proceduralmesh (Transformation|GetWorldRotation (Variables|/Game/__Actor/BP_VR_Slice_v1.BP_VR_Slice_v1_C|GetCamera _asbp_vr_slice_v_1)) false false)))

(fn ConstructionScript
  (|CallParentFunction))