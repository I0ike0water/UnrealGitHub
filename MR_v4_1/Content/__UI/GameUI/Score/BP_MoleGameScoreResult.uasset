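; BP_MoleGameScoreResult is an actor that shows the mole game's final score through a widget component and handles the clear condition.
; On BeginPlay it reads FirstGameScore from BP_GameInstance and passes it to the WBP_MoleGameScoreResult widget.
; If the score exceeds a hard-coded threshold, it spawns an actor at a fixed transform and calls the mole game clear event.
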(event EventBeginPlay
  (bind _asbp_game_instance (Utilities|Casting|CastToBP_GameInstance (Game|GetGameInstance)))
  (bind _aswbp_mole_game_score_result (Utilities|Casting|CastToWBP_MoleGameScoreResult (UserInterface|GetWidget (Variables|Default|GetWidget))))
  (Default|SetScoreValue _aswbp_mole_game_score_result (Variables|/Game/__GameInstance/BP_GameInstance.BP_GameInstance_C|GetFirstGameScore _asbp_game_instance))
  (if (< 49.0 (Variables|/Game/__GameInstance/BP_GameInstance.BP_GameInstance_C|GetFirstGameScore _asbp_game_instance))
    (Game|SpawnActorfromClass "/Game/__UI/GameUI/Guitar/BP_Clear.BP_Clear_C" (Math|Transform|MakeTransform "370.000000,-760.000000,100.000000" "0.000000,90.000000,0.000000" "1.000000,1.000000,1.000000") "AlwaysSpawn" "MultiplyWithRoot" 0 0)
    (Default|CallMoleGameClearEvent)))

(event Collision|EventActorBeginOverlap
  (params (OtherActor :type Actor%20Object%20Reference)))

(event EventTick
  (params (DeltaSeconds :type Float%20%28single-precision%29)))

(fn ConstructionScript)