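; BP_PhysicalInfo is an actor that displays the player's physical measurements through a WBP_PhysicalInfo widget.
; On BeginPlay it hides itself, then copies height, sitting height and wingspan from BP_GameInstance into the widget as text, adding a fixed offset to the wingspan.
; It becomes visible only if both the first and second game scores exceed a threshold, checked once at BeginPlay.
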(event EventBeginPlay
  (Rendering|SetActorHiddenInGame true)
  (bind _asbp_game_instance (Utilities|Casting|CastToBP_GameInstance (Game|GetGameInstance)))
  (bind _aswbp_physical_info (Utilities|Casting|CastToWBP_PhysicalInfo (UserInterface|GetWidget (Variables|Default|GetWidget))))
  (Variables|/Game/__UI/GameUI/InfoUI/WBP_PhysicalInfo.WBP_PhysicalInfo_C|SetHeightValue _aswbp_physical_info (Utilities|String|ToString(Float) (Variables|/Game/__GameInstance/BP_GameInstance.BP_GameInstance_C|GetHeight _asbp_game_instance)))
  (Variables|/Game/__UI/GameUI/InfoUI/WBP_PhysicalInfo.WBP_PhysicalInfo_C|SetSittingHeightValue _aswbp_physical_info (Utilities|String|ToString(Float) (Variables|/Game/__GameInstance/BP_GameInstance.BP_GameInstance_C|GetSittingHeight _asbp_game_instance)))
  (Variables|/Game/__UI/GameUI/InfoUI/WBP_PhysicalInfo.WBP_PhysicalInfo_C|SetWingSpanValue _aswbp_physical_info (Utilities|String|ToString(Float) (+ (Variables|/Game/__GameInstance/BP_GameInstance.BP_GameInstance_C|GetWingSpan _asbp_game_instance) 25.0)))
  (bind _asbp_game_instance_2 (Utilities|Casting|CastToBP_GameInstance (Game|GetGameInstance)))
  (if (< 49.0 (Variables|/Game/__GameInstance/BP_GameInstance.BP_GameInstance_C|GetFirstGameScore _asbp_game_instance_2))
    (if (< 49.0 (Variables|/Game/__GameInstance/BP_GameInstance.BP_GameInstance_C|GetSecondGameScore _asbp_game_instance_2))
      (Rendering|SetActorHiddenInGame false))))

(fn ConstructionScript)