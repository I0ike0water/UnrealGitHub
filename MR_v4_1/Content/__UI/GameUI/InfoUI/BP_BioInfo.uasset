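; BP_BioInfo is an in-game info actor that displays the player's biological age through a WBP_BiologicalAge widget component.
; It starts hidden in game on BeginPlay.
; Its BiologicalUpdate event copies PhysicsAge from BP_GameInstance into the widget's BioValue as text, then shows the actor only when that age is above zero.
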(event Custom|Biological%20Update
  (bind _asbp_game_instance (Utilities|Casting|CastToBP_GameInstance (Game|GetGameInstance)))
  (bind _aswbp_biological_age (Utilities|Casting|CastToWBP_BiologicalAge (UserInterface|GetWidget (Variables|Default|GetWidget))))
  (Variables|/Game/__UI/GameUI/InfoUI/WBP_BiologicalAge.WBP_BiologicalAge_C|SetBioValue _aswbp_biological_age (Utilities|String|ToString(Integer) (Variables|/Game/__GameInstance/BP_GameInstance.BP_GameInstance_C|GetPhysicsAge _asbp_game_instance)))
  (if (> (Variables|/Game/__GameInstance/BP_GameInstance.BP_GameInstance_C|GetPhysicsAge _asbp_game_instance) 0)
    (Rendering|SetActorHiddenInGame false)
    (else
      (Rendering|SetActorHiddenInGame true))))

(event EventBeginPlay
  (Rendering|SetActorHiddenInGame true))

(fn ConstructionScript)